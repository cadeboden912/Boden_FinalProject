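; Keypad lock for a door puzzle that opens a passcode widget and responds when the correct code is entered.
; CommunciatewithMe creates the Keypad widget, passes itself as LockBP and switches the player to UI-only input with a visible cursor.
; The correct-passcode event notifies DoorBP and plays a timeline that rotates the Cube.
; A one-second Delay driven from that timeline's Update starts a second timeline that slides the Cube.
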(event `/Game/FirstPersonBP/Blueprints/Communicate.CommunciateWithMe`
  (bind _returnvalue (`GameplayStatics.GetPlayerController` 0))
  ;[1 1 1] widget and incorrect passcode
  (bind _returnvalue_2 (`|CreateWidget` "/Game/AAGAM3362/01_Door_Puzzle/Cade_Door_Puzzle/Boden_Resources/Boden_Widgets/Keypad.Keypad_C"))
  (set `/Game/AAGAM3362/01_Door_Puzzle/Cade_Door_Puzzle/Boden_Resources/Boden_Widgets/Keypad.lock_BP` self _returnvalue_2)
  (`UserWidget.AddToViewport` _returnvalue_2 0)
  (`WidgetBlueprintLibrary.SetInputMode_UIOnlyEx` _returnvalue _returnvalue_2)
  (set `PlayerController.bShowMouseCursor` true _returnvalue))

(event `PAsscode:Correct`
  ;[1 1 1] password correct
  (`/Game/AAGAM3362/01_Door_Puzzle/Cade_Door_Puzzle/Boden_Resources/Cade_Blueprints/Boden_SlideDoor_lock.enter password:correect` (`self.Door_BP`))
  (bind (_direction _slide) (`Timeline|Timeline_0`)
    (:`Update`
      (`SceneComponent.K2_SetRelativeRotation` (`self.Cube`) (`KismetMathLibrary.RLerp` (`self.vault default`) (`self.vault new`) _slide) false false)
      (`KismetSystemLibrary.Delay` 1.0)
      (bind (_direction_2 _slide_2) (`Timeline|Timeline_1`)
        (:`Update`
          (`SceneComponent.K2_SetRelativeLocation` (`self.Cube`) (`KismetMathLibrary.VLerp` (`self.current`) (`self.New_Current`) _slide_2) false false))))))

(fn `UserConstructionScript`)