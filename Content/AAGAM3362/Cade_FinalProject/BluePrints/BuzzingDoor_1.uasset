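; BuzzingDoor_1 is a door actor that flickers and then destroys itself once something overlaps its Box trigger.
; The overlap starts a delay-driven loop that sets the Cube's material, then briefly hides and reshows the actor, counting each pass.
; After two passes it destroys the actor; the overlap has no actor filter or re-entry guard.
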(event `self.Box.OnComponentBeginOverlap`
  (params (OverlappedComponent :type "PrimitiveComponent Object Reference") (OtherActor :type "Actor Object Reference") (OtherComp :type "PrimitiveComponent Object Reference") (OtherBodyIndex :type Integer) (bFromSweep :type Boolean) (SweepResult :type "HitResult Structure (by ref)"))
  (`KismetSystemLibrary.Delay` 0.5 :!label _label)
  (if (>= (`self.loopcount`) 2)
    (`self.K2_DestroyActor`)
    (else
      (`PrimitiveComponent.SetMaterial` (`self.Cube`) 0 "/Game/AAGAM3362/Cade_FinalProject/material/data.data")
      (`KismetSystemLibrary.Delay` 0.5)
      (`self.SetActorHiddenInGame` true)
      (`KismetSystemLibrary.Delay` 0.1)
      (`self.SetActorHiddenInGame` false)
      (set `self.loopcount` (+ (`self.loopcount`) 1))
      (goto _label))))

(fn `UserConstructionScript`)