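; ToSecondFloor is an actor Blueprint with a Cube and a Button, apparently meant as a door opening to the second floor.
; Its construction script places the Button from a ButtonTransform variable.
; The event graph holds a timeline-driven slide of the Cube and a delayed material-swap and blink loop ending in actor destruction.
; None of these event graph chains has a triggering event, so they never run.
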(fn `UserConstructionScript`
  (`SceneComponent.K2_SetRelativeTransform` (`self.button`) (`self.Button_transform`) false false))