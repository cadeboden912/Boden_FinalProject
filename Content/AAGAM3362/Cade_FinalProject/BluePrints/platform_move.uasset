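; Moving platform actor that shuttles its Cube back and forth between OldLocation and NewLocation from BeginPlay.
; Two timelines lerp the relative location with sweep, one for each direction.
; Delays hang off each timeline's Update rather than Finished, so their timing counts from movement start.
; Rewind is cleared just before its check, so the outbound timeline always restarts; a third timeline branch is disconnected.
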(event `self.ReceiveBeginPlay`
  (bind (_direction _newtrack_0) (`Timeline|Timeline_0` :!label _label)
    (:`Update`
      (`SceneComponent.K2_SetRelativeLocation` (`self.Cube`) (`KismetMathLibrary.VLerp` (`self.old location`) (`self.new location`) _newtrack_0) true false)
      (`KismetSystemLibrary.Delay` 3.0)
      (bind (_direction_2 _newtrack_0_2) (`Timeline|Timeline_2`)
        (:`Update`
          (`SceneComponent.K2_SetRelativeLocation` (`self.Cube`) (`KismetMathLibrary.VLerp` (`self.new location`) (`self.old location`) _newtrack_0_2) true false)
          (set `self.Rewind` false)
          (`KismetSystemLibrary.Delay` 2.0)
          (if (not (`self.Rewind`))
            (goto _label :!via `PlayFromStart`)))))))

(fn `UserConstructionScript`)