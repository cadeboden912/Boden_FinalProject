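; EnemySpawner21 is an enemy spawner that places AI-controlled Enemy_Character1 pawns at random points inside its SpawnVolume box.
; Its SpawnEnemy event spawns one enemy only while the world count of that class is below MaxEnemies, then prints a debug string.
; Nothing in this graph calls SpawnEnemy, as BeginPlay, overlap and Tick are unused.
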(event `SpawnEnemy`
  (bind _outactors (`GameplayStatics.GetAllActorsOfClass` "/Game/Blueprints/Enemy_Character1.Enemy_Character1_C"))
  (if (< (`KismetArrayLibrary.Array_Length` _outactors) (`self.MaxEnemies`))
    (`AIBlueprintHelperLibrary.SpawnAIFromClass` "/Game/Blueprints/Enemy_Character1.Enemy_Character1_C" null (`KismetMathLibrary.RandomPointInBoundingBox` (`SceneComponent.K2_GetComponentLocation` (`self.SpawnVolume`)) (`BoxComponent.GetScaledBoxExtent` (`self.SpawnVolume`))) (struct) false null)
    (`KismetSystemLibrary.PrintString` "HI")))

(fn `UserConstructionScript`)